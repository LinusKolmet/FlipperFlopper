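; Player character for Flipper Flopper, a platformer with coyote-time jumps, hold-to-bunny-hop and a speed-gated belly flop that launches along Y with altered ground friction.
; Capsule overlaps dispatch by actor tag to collect items, activate a single checkpoint, flag a win, or trigger death.
; Death, also bound to the B key, plays an orca kill animation, then respawns at the current checkpoint or restarts the level.
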(event OnComponentBeginOverlap(CapsuleComponent)
  (params (OverlappedComponent :type Primitive%20Component%20Object%20Reference) (OtherActor :type Actor%20Object%20Reference) (OtherComp :type Primitive%20Component%20Object%20Reference) (OtherBodyIndex :type Integer) (bFromSweep :type Boolean) (SweepResult :type Hit%20Result%20Structure%20%28by%20ref%29))
  (bind _returnvalue (Transformation|GetActorLocation))
  (bind _charactermovement (Variables|Character|GetCharacterMovement))
  ;[1 1 1] collectible overlap
  (if (Actor|ActorHasTag OtherActor "Collectible")
    (bind _output_get (Variables|Default|SetCurrentCollectible OtherActor))
    (Audio|PlaySoundatLocation "/Game/Programming/Sound/Metasounds/Collecting.Collecting" (Transformation|GetActorLocation _output_get) "0, 0, 0" 1.0 1.0 0.0 0 0 0 0)
    (Variables|Default|SetAmountCollectibles (+ (Variables|Default|GetAmountCollectibles) 1))
    (Actor|DestroyActor _output_get)
    (else
      ;[1 1 1] checkpoint overlap
      (if (Actor|ActorHasTag OtherActor "Checkpoint")
        (Variables|Default|SetCurrentCheckpoint OtherActor)
        (Variables|Default|SetHasReachedAnyCheckpoint true)
        (bind _outactors (Actor|GetAllActorsOfClass "/Game/Programming/BP_Checkpoint_V2.BP_Checkpoint_V2_C"))
        (for _array_element _outactors
          (if (== _array_element (Variables|Default|GetCurrentCheckpoint))
            (Default|Activate _array_element)
            (else
              (Default|Deactivate _array_element))))
        (else
          ;[1 1 1] deathbox overlap
          (if (Actor|ActorHasTag OtherActor "Deathbox")
            (bind _asflipper_flopper_game_mode (Utilities|Casting|CastToFlipperFlopperGameMode (Game|GetGameMode)))
            (Variables|/Game/Programming/FlipperFlopperGameMode.FlipperFlopperGameMode_C|SetPlayerIsLoser _asflipper_flopper_game_mode true)
            (bind _returnvalue_2 (Game|SpawnActorfromClass "/Game/Programming/BP_Orca.BP_Orca_C" (Math|Transform|MakeTransform (Math|Vector|MakeVector (.x _returnvalue) (.y _returnvalue) (- (.z _returnvalue) 1.5e+02)) "0.000000,180.000000,0.000000" "1.000000,1.000000,1.000000") "Undefined" "OverrideRootScale" 0 0))
            (Pawn|Components|CharacterMovement|DisableMovement _charactermovement)
            (Rendering|SetVisibility (Variables|Character|GetMesh) false false)
            (Components|Animation|PlayAnimation (Variables|/Game/Programming/BP_Orca.BP_Orca_C|GetbMesh_KillerOrca_v4 _returnvalue_2) "/Game/Assets/Temporary/Orca/bMesh_KillerOrca_v4_Anim_Kill_002.bMesh_KillerOrca_v4_Anim_Kill_002" false)
            (Utilities|FlowControl|Delay 3.2)
            (CallFunction|Respawn)
            (Pawn|Components|CharacterMovement|SetMovementMode _charactermovement "MOVE_Walking" 0)
            (Actor|DestroyActor _returnvalue_2)
            (Rendering|SetVisibility (Variables|Character|GetMesh) true false)
            (else
              ;[1 1 1] win area overlap
              (if (Actor|ActorHasTag OtherActor "Winarea")
                (bind _asflipper_flopper_game_mode_2 (Utilities|Casting|CastToFlipperFlopperGameMode (Game|GetGameMode)))
                (Variables|/Game/Programming/FlipperFlopperGameMode.FlipperFlopperGameMode_C|SetPlayerIsWinner _asflipper_flopper_game_mode_2 true)))))))))

(event Custom|CoyoteTimerOut
  ;[1 1 1] bHop
)

(event Custom|Respawn
  ;[1 1 1] Respawn
  (if (Variables|Default|GetHasReachedAnyCheckpoint)
    (bind _outactors (Actor|GetAllActorsOfClass "/Game/Programming/BP_Checkpoint_V2.BP_Checkpoint_V2_C"))
    (bind _array_element (Utilities|Array|ForEachLoopwithBreak _outactors)
      (:LoopBody
        (if (== _array_element (Variables|Default|GetCurrentCheckpoint))
          (CallFunction|CheckpointBreak)))
      (:Completed
        (Transformation|SetActorLocation (Transformation|GetWorldLocation (Variables|/Game/Programming/BP_Checkpoint_V2.BP_Checkpoint_V2_C|GetTPPoint _array_element)) false false)))
    (else
      (bind _asmain_character_player_controller (Utilities|Casting|CastToMainCharacterPlayerController (Game|GetPlayerController 0)))
      (Default|RestartLevel _asmain_character_player_controller false))))

(event Custom|Checkpoint%20Break
  ;[1 1 1] Respawn
  (Utilities|Array|ForEachLoopwithBreak (stale Custom|Respawn _outactors)) ; enters at Break
)

(event EventBeginPlay
  (Variables|Default|SetHasReachedAnyCheckpoint false)
  (Variables|Default|SetFriction%20resetter (Variables|/Script/Engine.CharacterMovementComponent|GetGroundFriction (Variables|Character|GetCharacterMovement))))

(event EventTick
  (params (DeltaSeconds :type Float%20%28single-precision%29))
  (bind _charactermovement (Variables|Character|GetCharacterMovement))
  (if (Variables|Default|GetBellyFlopActive)
    (if (<= (Math|Float|Absolute(Float) (.y (Transformation|GetVelocity))) (Variables|/Script/Engine.CharacterMovementComponent|GetMaxWalkSpeed _charactermovement))
      (Variables|/Script/Engine.CharacterMovementComponent|SetGroundFriction _charactermovement (Variables|Default|GetFriction%20resetter))
      (Variables|Default|SetBellyFlopActive false))))

(event EventOnMovementModeChanged
  (params (PrevMovementMode :type EMovementMode%20Enum :default "MOVE_None") (NewMovementMode :type EMovementMode%20Enum :default "MOVE_None") (PrevCustomMode :type Byte :default 0) (NewCustomMode :type Byte :default 0))
  ;[1 1 1] Bunny Hop
  (if (Utilities|Enum|Equal(Enum) NewMovementMode "MOVE_Walking")
    (bind _asmain_character_player_controller (Utilities|Casting|CastToMainCharacterPlayerController (Game|GetPlayerController 0)))
    (if (Game|Player|IsInputKeyDown _asmain_character_player_controller "SpaceBar")
      (Character|Jump))
    (else
      ;[1 1 1] bHop
      (if (and (Utilities|Enum|Equal(Enum) PrevMovementMode "MOVE_Walking") (Utilities|Enum|Equal(Enum) NewMovementMode "MOVE_Falling"))
        (bind _returnvalue (Utilities|Time|SetTimerbyEvent (delegate Custom|CoyoteTimerOut) (Variables|Default|GetCoyoteTime)))
        (Variables|Default|SetCoyoteTimer _returnvalue)))))

(event EventOnLanded
  (params (Hit :type Hit%20Result%20Structure%20%28by%20ref%29))
  ;[1 1 1] bHop
  (Utilities|Time|ClearandInvalidateTimerbyHandle (Variables|Default|GetCoyoteTimer))
  (bind _asmain_character_player_controller (Utilities|Casting|CastToMainCharacterPlayerController (Pawn|GetController)))
  (Default|OnCharacterLand _asmain_character_player_controller))

(event Input|KeyboardEvents|B
  (params (Key :type Key%20Structure :default "None"))
  (bind _returnvalue (Transformation|GetActorLocation))
  (bind _charactermovement (Variables|Character|GetCharacterMovement))
  ;[1 1 1] deathbox overlap
  (:Pressed
    (bind _asflipper_flopper_game_mode (Utilities|Casting|CastToFlipperFlopperGameMode (Game|GetGameMode)))
    (Variables|/Game/Programming/FlipperFlopperGameMode.FlipperFlopperGameMode_C|SetPlayerIsLoser _asflipper_flopper_game_mode true)
    (bind _returnvalue_2 (Game|SpawnActorfromClass "/Game/Programming/BP_Orca.BP_Orca_C" (Math|Transform|MakeTransform (Math|Vector|MakeVector (.x _returnvalue) (.y _returnvalue) (- (.z _returnvalue) 1.5e+02)) "0.000000,180.000000,0.000000" "1.000000,1.000000,1.000000") "Undefined" "OverrideRootScale" 0 0))
    (Pawn|Components|CharacterMovement|DisableMovement _charactermovement)
    (Rendering|SetVisibility (Variables|Character|GetMesh) false false)
    (Components|Animation|PlayAnimation (Variables|/Game/Programming/BP_Orca.BP_Orca_C|GetbMesh_KillerOrca_v4 _returnvalue_2) "/Game/Assets/Temporary/Orca/bMesh_KillerOrca_v4_Anim_Kill_002.bMesh_KillerOrca_v4_Anim_Kill_002" false)
    (Utilities|FlowControl|Delay 3.2)
    (CallFunction|Respawn)
    (Pawn|Components|CharacterMovement|SetMovementMode _charactermovement "MOVE_Walking" 0)
    (Actor|DestroyActor _returnvalue_2)
    (Rendering|SetVisibility (Variables|Character|GetMesh) true false)))

(fn ConstructionScript
  (|CallParentFunction))

(fn CanJumpInternal
  (bind _returnvalue (|CallParentFunction))
  (return (or _returnvalue (> (Utilities|Time|GetTimerRemainingTimebyHandle (Variables|Default|GetCoyoteTimer)) 0.0))))

(fn BellyFlop
  (bind _returnvalue (Transformation|GetVelocity))
  (if (not (Variables|Default|GetBellyFlopActive))
    (if (>= (Math|Float|Absolute(Float) (.y _returnvalue)) (* (Variables|/Script/Engine.CharacterMovementComponent|GetMaxWalkSpeed (Variables|Character|GetCharacterMovement)) (Variables|Default|GetBellyFlopRequiredMovementspeedPercentage)))
      (bind _output_get (Variables|Default|SetBellyFlopActive true))
      (Development|PrintText (Utilities|Text|ToText(Boolean) _output_get))
      (Variables|/Script/Engine.CharacterMovementComponent|SetGroundFriction (Variables|Character|GetCharacterMovement) (Variables|Default|GetBellyFlopGroundFriction))
      (if (> (.y _returnvalue) 0.0)
        (Character|LaunchCharacter (Math|Vector|MakeVector 0.0 (Variables|Default|GetBellyFlopLaunch) 0.0) false false)
        (else
          (Character|LaunchCharacter (Math|Vector|MakeVector 0.0 (- 0.0 (Variables|Default|GetBellyFlopLaunch)) 0.0) false false))))))